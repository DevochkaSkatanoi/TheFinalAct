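; BP_Samael is the player character, with movement, sprint, sphere-overlap interaction and unlockable masks selected by input.
; Equipping a mask notifies all BPI_MaskEffect actors, updates the HUD and grants a double jump for the fourth mask.
; A CanJumpInternal override adds delayed coyote time and a downward-trace landing buffer.
; Falling too long triggers a camera-fade respawn at the GameInstance's spawn transform, also applied on BeginPlay.
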(event Custom|Respawn
  ;[0.15 0.06647 0 0.5] Respawn
  (Utilities|FlowControl|DoOnce false :!label _label
    (:Completed
      (CameraFades|StartCameraFade :self (Game|GetPlayerCameraManager 0) :ToAlpha 1.0 :Duration 1.0 :bHoldWhenFinished true)
      (Utilities|FlowControl|Delay 2.0)
      (CallFunction|TeleporttoSpawn)
      (CameraFades|StartCameraFade :self (Game|GetPlayerCameraManager 0) :FromAlpha 1.0 :Duration 1.0)
      (goto _label Reset))))

(event Custom|Sprint
  (bind _charactermovement (Variables|Character|GetCharacterMovement))
  ;[0.15 0.02918 0 0.5] Sprint
  (CallFunction|ResetIffallingTooLong)
  (if (and (Variables|Default|GetWantsToSprint) (AI|Components|NavMovement|IsMovingonGround (Variables|Character|GetCharacterMovement)))
    (Variables|/Script/Engine.CharacterMovementComponent|SetMaxWalkSpeed _charactermovement (Variables|Default|GetSpeed_Sprint))
    (else
      (Variables|/Script/Engine.CharacterMovementComponent|SetMaxWalkSpeed _charactermovement (Variables|Default|GetSpeed_Walk)))))

(event Custom|BufferTime
  (bind _returnvalue (Transformation|GetActorLocation))
  (bind _charactermovement (Variables|Character|GetCharacterMovement))
  (bind _velocity (Variables|/Script/Engine.MovementComponent|GetVelocity _charactermovement))
  ;[0.15 0.1357 0 0.5] Buffer Time
  (Utilities|FlowControl|Sequence
    (:then_0
      (if (< (.z _velocity) 0.0)
        (bind _returnvalue_2 (Collision|LineTraceByChannel _returnvalue (- _returnvalue "0.000000,0.000000,100.000000") "TraceTypeQuery1" false 0 "None"))
        (if _returnvalue_2
          (Variables|Default|SetbCanJump true))))
    (:then_1
      (if (> (.z _velocity) 0.0)
        (if (Utilities|Enum|Equal(Enum) (Variables|Masken|GetCurrentMask) "NewEnumerator3")
          (Variables|Default|SetbCanJump true)
          (else
            (Variables|Default|SetbCanJump false)))))))

(event Input|EnhancedActionEvents|EnhancedInputActionIA_Move
  (params (ActionValue :type Vector%202D%20Structure) (ElapsedSeconds :type Float%20%28double-precision%29) (TriggeredSeconds :type Float%20%28double-precision%29) (InputAction :type Input%20Action%20Object%20Reference :default "/Game/Input/Actions/IA_Move.IA_Move"))
  ;[0.15 0.004816 0.003241 0.5] Input Actions
  (CallFunction|MoveLocalDirection (.x ActionValue) (.y ActionValue)))

(event Input|EnhancedActionEvents|EnhancedInputActionIA_Look
  (params (ActionValue :type Vector%202D%20Structure) (ElapsedSeconds :type Float%20%28double-precision%29) (TriggeredSeconds :type Float%20%28double-precision%29) (InputAction :type Input%20Action%20Object%20Reference :default "/Game/Input/Actions/IA_Look.IA_Look"))
  ;[0.15 0.004816 0.003241 0.5] Input Actions
  (Pawn|Input|AddControllerYawInput (.x ActionValue))
  (Pawn|Input|AddControllerPitchInput (.y ActionValue)))

(event Input|EnhancedActionEvents|EnhancedInputActionIA_Jump
  (params (ActionValue :type Boolean) (ElapsedSeconds :type Float%20%28double-precision%29) (TriggeredSeconds :type Float%20%28double-precision%29) (InputAction :type Input%20Action%20Object%20Reference :default "/Game/Input/Actions/IA_Jump.IA_Jump"))
  ;[0.15 0.004816 0.003241 0.5] Input Actions
  (:Triggered
    (Utilities|FlowControl|DoOnce false :!label _label
      (:Completed
        (Character|Jump))))
  (:Completed
    (Character|StopJumping)
    (goto _label Reset)))

(event Input|EnhancedActionEvents|EnhancedInputActionIA_Sprint
  (params (ActionValue :type Boolean) (ElapsedSeconds :type Float%20%28double-precision%29) (TriggeredSeconds :type Float%20%28double-precision%29) (InputAction :type Input%20Action%20Object%20Reference :default "/Game/Input/Actions/IA_Sprint.IA_Sprint"))
  ;[0.15 0.004816 0.003241 0.5] Input Actions
  (:Triggered
    (Variables|Default|SetWantsToSprint true))
  (:Completed
    (Variables|Default|SetWantsToSprint false)))

(event Input|EnhancedActionEvents|EnhancedInputActionIA_Interact
  (params (ActionValue :type Boolean) (ElapsedSeconds :type Float%20%28double-precision%29) (TriggeredSeconds :type Float%20%28double-precision%29) (InputAction :type Input%20Action%20Object%20Reference :default "/Game/Input/Actions/IA_Interact.IA_Interact"))
  ;[0.15 0.004816 0.003241 0.5] Input Actions
  ;;[0.15 0 0.0688 0.5] Interact
  (bind (_outactors _returnvalue) (Collision|SphereOverlapActors (+ (* (Transformation|GetActorForwardVector) 1.5e+02) (Transformation|GetActorLocation)) (Math|Float|MakeLiteralFloat 1e+02) (Utilities|Array|MakeArray "ObjectTypeQuery1" "ObjectTypeQuery2" "ObjectTypeQuery3" "ObjectTypeQuery4") 0 (Utilities|Array|MakeArray self)))
  (for _array_element _outactors
    (if (Utilities|DoesObjectImplementInterface _array_element "/Game/BP/Interactables/IInteractable.IInteractable_C")
      (Class|IInteractable|Interact(Message) _array_element))))

(event Input|EnhancedActionEvents|EnhancedInputActionIA_Pause
  (params (ActionValue :type Boolean) (ElapsedSeconds :type Float%20%28double-precision%29) (TriggeredSeconds :type Float%20%28double-precision%29) (InputAction :type Input%20Action%20Object%20Reference :default "/Game/Input/Actions/IA_Pause.IA_Pause"))
  ;[0.15 0.004816 0.003241 0.5] Input Actions
  (bind _asbp_hud (Utilities|Casting|CastToBP_HUD (HUD|GetHUD (Game|GetPlayerController 0))))
  (Default|Pause _asbp_hud))

(event Input|EnhancedActionEvents|EnhancedInputActionIA_Mask_1
  (params (ActionValue :type Boolean) (ElapsedSeconds :type Float%20%28double-precision%29) (TriggeredSeconds :type Float%20%28double-precision%29) (InputAction :type Input%20Action%20Object%20Reference :default "/Game/Input/Actions/IA_Mask_1.IA_Mask_1"))
  ;[0.15 0.004816 0.003241 0.5] Input Actions
  (CallFunction|TrySelectMask "NewEnumerator0"))

(event Input|EnhancedActionEvents|EnhancedInputActionIA_Mask_2
  (params (ActionValue :type Boolean) (ElapsedSeconds :type Float%20%28double-precision%29) (TriggeredSeconds :type Float%20%28double-precision%29) (InputAction :type Input%20Action%20Object%20Reference :default "/Game/Input/Actions/IA_Mask_2.IA_Mask_2"))
  ;[0.15 0.004816 0.003241 0.5] Input Actions
  (CallFunction|TrySelectMask "NewEnumerator1"))

(event Input|EnhancedActionEvents|EnhancedInputActionIA_Mask_3
  (params (ActionValue :type Boolean) (ElapsedSeconds :type Float%20%28double-precision%29) (TriggeredSeconds :type Float%20%28double-precision%29) (InputAction :type Input%20Action%20Object%20Reference :default "/Game/Input/Actions/IA_Mask_3.IA_Mask_3"))
  ;[0.15 0.004816 0.003241 0.5] Input Actions
  (CallFunction|TrySelectMask "NewEnumerator2"))

(event Input|EnhancedActionEvents|EnhancedInputActionIA_Mask_4
  (params (ActionValue :type Boolean) (ElapsedSeconds :type Float%20%28double-precision%29) (TriggeredSeconds :type Float%20%28double-precision%29) (InputAction :type Input%20Action%20Object%20Reference :default "/Game/Input/Actions/IA_Mask_4.IA_Mask_4"))
  ;[0.15 0.004816 0.003241 0.5] Input Actions
  (CallFunction|TrySelectMask "NewEnumerator3"))

(event EventBeginPlay
  ;[0.15 0.004816 0.003241 0.5] Input Actions
  (CallFunction|TeleporttoSpawn)
  (Input|AddMappingContext (PlayerController|LocalPlayerSubsystems|GetEnhancedInputLocalPlayerSubsystem (Game|GetPlayerController 0)) "/Game/Input/IMC_Player.IMC_Player" 0 "(bIgnoreAllPressedKeysUntilRelease=True,bForceImmediately=False,bNotifyUserSettings=False)")
  (CameraFades|StartCameraFade :self (Game|GetPlayerCameraManager 0) :FromAlpha 1.0 :Duration 2.0))

(event EventOnMovementModeChanged
  (params (PrevMovementMode :type EMovementMode%20Enum :default "MOVE_None") (NewMovementMode :type EMovementMode%20Enum :default "MOVE_None") (PrevCustomMode :type Byte :default 0) (NewCustomMode :type Byte :default 0))
  ;[0.15 0.08028 0 0.5] Coyote Time
  (if (Utilities|Enum|Equal(Enum) NewMovementMode "MOVE_Walking")
    (Variables|Default|SetbCanJump true)
    (elif (Utilities|Enum|Equal(Enum) NewMovementMode "MOVE_Falling")
      (if (<= (.z (Variables|/Script/Engine.MovementComponent|GetVelocity (Variables|Character|GetCharacterMovement))) 0.0)
        (Utilities|FlowControl|Delay 0.3)
        (if (Utilities|Enum|Equal(Enum) (Variables|/Script/Engine.CharacterMovementComponent|GetMovementMode (Variables|Character|GetCharacterMovement)) "MOVE_Falling")
          (Variables|Default|SetbCanJump false))
        (else
          (Variables|Default|SetbCanJump false))))))

(event EventTick
  (params (DeltaSeconds :type Float%20%28single-precision%29))
  ;[0.15 0.15 0.15 0.5] Event Tick
  (CallFunction|Sprint)
  (CallFunction|BufferTime))

(fn ConstructionScript
  (Variables|/Script/Engine.CharacterMovementComponent|SetMaxWalkSpeed (Variables|Character|GetCharacterMovement) (Variables|Default|GetSpeed_Walk)))

(fn MoveLocalDirection
  (params (WorldDirection_X :type Float%20%28double-precision%29) (WorldDirection_Y :type Float%20%28double-precision%29))
  (bind _camera (Variables|Default|GetCamera))
  (bind _returnvalue (Transformation|GetWorldTransform _camera))
  (Pawn|Input|AddMovementInput (Math|Transform|TransformDirection (Math|Transform|MakeTransform (.location _returnvalue) (Math|Rotator|MakeRotator 0.0 0.0 (.yaw (.rotation _returnvalue))) (.scale _returnvalue)) (Math|Vector|MakeVector WorldDirection_X WorldDirection_Y 0.0)) 1.0 false))

(fn TeleporttoSpawn
  (bind _asbp_game_instance (Utilities|Casting|CastToBP_GameInstance (Game|GetGameInstance))
    (:then
      (if (.HasValidPlayerTransform (Default|TryGetPlayerSpawnTransform _asbp_game_instance))
        (Transformation|SetActorLocationAndRotation (.location (.PlayerRespawnTransform (Default|TryGetPlayerSpawnTransform _asbp_game_instance))) (.rotation (.PlayerRespawnTransform (Default|TryGetPlayerSpawnTransform _asbp_game_instance))))))
    (:CastFailed
      (Development|PrintString "WRONG GAME INSTANCE" true true "(R=1.000000,G=0.044832,B=0.000000,A=1.000000)"))))

(fn ResetIffallingTooLong
  (if (AI|Components|NavMovement|IsMovingonGround (Variables|Character|GetCharacterMovement))
    (Variables|Default|SetLastGroundedTime (Utilities|Time|GetGameTimeinSeconds))
    (elif (> (- (Utilities|Time|GetGameTimeinSeconds) (Variables|Default|GetLastGroundedTime)) (Variables|Default|GetMaxFallDuration))
      (CallFunction|Respawn))))

(fn BroadcastMaskChange
  (bind _outactors (Actor|GetAllActorswithInterface "/Game/BP/Collectables/BPI_MaskEffect.BPI_MaskEffect_C"))
  (for _array_element _outactors
    (Class|BPIMaskEffect|OnMaskChanged(Message) _array_element (Variables|Masken|GetCurrentMask))))

(fn EquipMask
  (params (MaskType :type E_MaskType%20Enum :default "NewEnumerator0"))
  (bind _output_get (Variables|Masken|SetCurrentMask MaskType))
  (CallFunction|BroadcastMaskChange)
  (Variables|Default|SetJumpMaxCount (Math|Integer|SelectInt 2 1 (Utilities|Enum|Equal(Enum) _output_get "NewEnumerator3")))
  (bind _asbp_hud (Utilities|Casting|CastToBP_HUD (HUD|GetHUD (Game|GetPlayerController 0))))
  (Default|ShowImage (Variables|/Game/UI/BP_HUD.BP_HUD_C|GetMasks%20Widget _asbp_hud) (Variables|Masken|GetCurrentMask)))

(fn TrySelectMask
  (params (InputMask :type E_MaskType%20Enum :default "NewEnumerator0"))
  (if (Utilities|Set|Contains (Variables|Default|GetUnlockedMask) InputMask)
    (Development|PrintString "true")
    (CallFunction|EquipMask InputMask)
    (else
      (Development|PrintString "false"))))

(fn UnlockMask
  (params (MaskType :type E_MaskType%20Enum :default "NewEnumerator0"))
  (Utilities|Set|Add (Variables|Default|GetUnlockedMask) MaskType)
  (bind _asbp_hud (Utilities|Casting|CastToBP_HUD (HUD|GetHUD (Game|GetPlayerController 0))))
  (Default|UnlockMask (Variables|/Game/UI/BP_HUD.BP_HUD_C|GetMasks%20Widget _asbp_hud) MaskType))

(fn CanJumpInternal
  (return (Variables|Default|GetbCanJump)))