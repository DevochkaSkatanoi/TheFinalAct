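; BP_Disappearing_Tambourine is a tambourine platform that visually breaks when BP_Samael steps into its trigger box without a specific mask equipped.
; Overlap swaps the material to Mask, then after DisappearingTime changes the mesh to Broken_Tambourine.
; Any end overlap restores the white material and intact mesh after two seconds.
; Collision toggle calls exist but are unconnected, so the graph never changes collision settings directly.
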(event OnComponentBeginOverlap(Box)
  (params (OverlappedComponent :type Primitive%20Component%20Object%20Reference) (OtherActor :type Actor%20Object%20Reference) (OtherComp :type Primitive%20Component%20Object%20Reference) (OtherBodyIndex :type Integer) (bFromSweep :type Boolean) (SweepResult :type Hit%20Result%20Structure%20%28by%20ref%29))
  (bind _asbp_samael (Utilities|Casting|CastToBP_Samael OtherActor))
  (if (not (Utilities|Enum|Equal(Enum) (Variables|/Game/Samael/BP_Samael.BP_Samael_C|GetCurrentMask _asbp_samael) "NewEnumerator1"))
    (Rendering|Material|SetMaterial (Variables|Default|GetPlatform) 0 "/Game/Samael/Materials/Mask.Mask")
    (Utilities|FlowControl|Delay (Variables|Default|GetDisappearingTime))
    (Components|StaticMesh|SetStaticMesh (Variables|Default|GetPlatform) "/Game/Assets/Final_Assets/Broken_Tambourine.Broken_Tambourine")))

(event OnComponentEndOverlap(Box)
  (params (OverlappedComponent :type Primitive%20Component%20Object%20Reference) (OtherActor :type Actor%20Object%20Reference) (OtherComp :type Primitive%20Component%20Object%20Reference) (OtherBodyIndex :type Integer))
  (Utilities|FlowControl|Delay 2.0)
  (Rendering|Material|SetMaterial (Variables|Default|GetPlatform) 0 "/Game/Materials/M_White.M_White")
  (Components|StaticMesh|SetStaticMesh (Variables|Default|GetPlatform) "/Game/Assets/Final_Assets/P_Tambourine.P_Tambourine"))

(fn ConstructionScript)