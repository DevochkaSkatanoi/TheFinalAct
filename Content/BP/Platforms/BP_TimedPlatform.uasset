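; BP_TimedPlatform is a platform that repeatedly appears and disappears on a timer.
; BeginPlay starts the Toggle event, which waits for Time, then shows the Mesh with query and physics collision.
; After the Visible delay it hides the Mesh, disables collision and calls itself again to loop indefinitely.
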(event Custom|Toggle
  (Utilities|FlowControl|Delay (Variables|Default|GetTime))
  (Rendering|SetVisibility (Variables|Default|GetMesh) true false)
  (Collision|SetCollisionEnabled (Variables|Default|GetMesh) "QueryAndPhysics")
  (Utilities|FlowControl|Delay (Variables|Default|GetVisible))
  (Rendering|SetVisibility (Variables|Default|GetMesh) false false)
  (Collision|SetCollisionEnabled (Variables|Default|GetMesh) "NoCollision")
  (CallFunction|Toggle))

(event EventBeginPlay
  (CallFunction|Toggle))

(fn ConstructionScript)