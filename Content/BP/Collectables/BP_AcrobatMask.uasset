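; BP_AcrobatMask is a collectable pickup that grants the player the acrobat mask.
; When a Character overlaps its Sphere, it disables collision on the sphere and mask, hides the mask, then flags the mask active and equips and unlocks it on the player.
; Tick keeps a timeline playing, whose CoinPath track drives the mask's yaw to animate it.
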(event OnComponentBeginOverlap(Sphere)
  (params (OverlappedComponent :type Primitive%20Component%20Object%20Reference) (OtherActor :type Actor%20Object%20Reference) (OtherComp :type Primitive%20Component%20Object%20Reference) (OtherBodyIndex :type Integer) (bFromSweep :type Boolean) (SweepResult :type Hit%20Result%20Structure%20%28by%20ref%29))
  (bind _player (Variables|Default|GetPlayer))
  (Utilities|Casting|CastToCharacter OtherActor)
  (Collision|SetCollisionEnabled (Variables|Default|GetSphere) "NoCollision")
  (Collision|SetCollisionEnabled (Variables|Default|GetMask) "NoCollision")
  (Rendering|SetVisibility (Variables|Default|GetMask) false false)
  (Variables|/Game/Samael/BP_Samael.BP_Samael_C|SetIsAcrMaskActive _player true)
  (Default|EquipMask _player "NewEnumerator3")
  (Default|UnlockMask _player "NewEnumerator3"))

(event EventTick
  (params (DeltaSeconds :type Float%20%28single-precision%29))
  (bind _coinpath (Timeline|Timeline Play)
    (:Update
      (Transformation|SetRelativeRotation (Variables|Default|GetMask) (Math|Rotator|MakeRotator 0.0 0.0 (* _coinpath 1e+02)) false false))))

(fn ConstructionScript)