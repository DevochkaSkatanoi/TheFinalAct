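; BP_Door is a swinging door that opens away from or toward BP_Samael, depending on the side they overlap its Box from.
; The character's local Y position sets the swing sign, and a timeline scales DoorOpenAngel by it to yaw the Piviot component.
; A CanChangeDirection flag locks that sign until the timeline finishes backward, though this graph only ever plays it forward.
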(event OnComponentBeginOverlap(Box)
  (params (OverlappedComponent :type Primitive%20Component%20Object%20Reference) (OtherActor :type Actor%20Object%20Reference) (OtherComp :type Primitive%20Component%20Object%20Reference) (OtherBodyIndex :type Integer) (bFromSweep :type Boolean) (SweepResult :type Hit%20Result%20Structure%20%28by%20ref%29))
  (bind _asbp_samael (Utilities|Casting|CastToBP_Samael OtherActor))
  (if (Variables|Default|GetCanChangeDirection)
    (Variables|Default|SetDir (Math|Float|SelectFloat 1.0 -1.0 (> (.y (Math|Transform|InverseTransformLocation (Transformation|GetActorTransform) (Transformation|GetActorLocation _asbp_samael))) 0.0)))
    (Variables|Default|SetCanChangeDirection false)
    (bind (_direction _rotation) (Timeline|Door_Open_Movement Play)
      (:Update
        (Transformation|SetRelativeRotation (Variables|Default|GetPiviot) (Math|Rotator|MakeRotator 0.0 0.0 (* _rotation (Variables|Default|GetDoorOpenAngel) (Variables|Default|GetDir))) false false))
      (:Finished
        (if (Utilities|Enum|Equal(Enum) _direction "Backward")
          (Variables|Default|SetCanChangeDirection true))))
    (else
      (Timeline|Door_Open_Movement Play))))

(fn ConstructionScript)