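; BP_Checkpoint is a checkpoint actor that updates the player's respawn point.
; When BP_Samael overlaps its Sphere, it passes the Arrow component's world transform to BP_GameInstance as the player spawn transform.
; GetRespawnRotation exposes the Arrow's forward vector, despite its name suggesting a rotation.
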(event OnComponentBeginOverlap(Sphere)
  (params (OverlappedComponent :type Primitive%20Component%20Object%20Reference) (OtherActor :type Actor%20Object%20Reference) (OtherComp :type Primitive%20Component%20Object%20Reference) (OtherBodyIndex :type Integer) (bFromSweep :type Boolean) (SweepResult :type Hit%20Result%20Structure%20%28by%20ref%29))
  (Utilities|Casting|CastToBP_Samael OtherActor)
  (bind _asbp_game_instance (Utilities|Casting|CastToBP_GameInstance (Game|GetGameInstance)))
  (Default|SetPlayerSpawnTransform _asbp_game_instance (Transformation|GetWorldTransform (Variables|Default|GetArrow))))

(fn ConstructionScript)

(fn GetRespawnRotation
  (return (Math|Rotator|GetRotationXVector (Transformation|GetWorldRotation (Variables|Default|GetArrow)))))