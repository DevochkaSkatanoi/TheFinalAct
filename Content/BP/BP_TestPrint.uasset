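; BP_TestPrint is a test actor that animates a mesh and a point light at runtime.
; On BeginPlay, the MeshMod event prints a debug string, moves, rotates and rescales MyMesh, swaps it to a pyramid mesh and tints the light.
; Tick raises the mesh continuously and, through a 0.2-second Delay, re-randomizes the light's color and its intensity within variable bounds, producing a disco-like flicker.
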(event Custom|MeshMod
  (bind _mymesh (Variables|Default|GetMyMesh))
  (bind _pointlight (Variables|Default|GetPointLight))
  (Development|PrintString "Blueprint")
  (Transformation|AddWorldOffset _mymesh "0.000000,0.000000,100.000000" false false)
  (Transformation|AddWorldRotation _mymesh "0.000000,45.000000,0.000000" false false)
  (Transformation|SetWorldScale3D _mymesh "0.500000,0.500000,2.000000")
  (Components|StaticMesh|SetStaticMesh _mymesh "/ControlRig/Controls/ControlRig_Pyramid_solid.ControlRig_Pyramid_solid")
  (Rendering|Components|Light|SetIntensity _pointlight 1e+02)
  (Rendering|Components|Light|SetLightColor _pointlight "(R=0.055231,G=0.768041,B=1.000000,A=1.000000)" true))

(event EventBeginPlay
  (CallFunction|MeshMod))

(event Collision|EventActorBeginOverlap
  (params (OtherActor :type Actor%20Object%20Reference))
  ;[0.15 0.04642 0.0653 0.5] Trigger and Collision
)

(event EventTick
  (params (DeltaSeconds :type Float%20%28single-precision%29))
  (Transformation|AddWorldOffset (Variables|Default|GetMyMesh) "0.000000,0.000000,1.000000" false false)
  (Utilities|FlowControl|Delay 0.2)
  (Rendering|Components|Light|SetIntensity (Variables|Default|GetPointLight) (Math|Random|RandomFloatinRange (Variables|Light|Get%20Lightintensity_Min) (Variables|Light|GetLightintensity_Max)))
  (Rendering|Components|Light|SetLightColor (Variables|Default|GetPointLight) (Utilities|Struct|MakeLinearColor (Math|Random|RandomFloat) (Math|Random|RandomFloat) (Math|Random|RandomFloat) 0.0) true))

(event Collision|EventHit
  (params (MyComp :type Primitive%20Component%20Object%20Reference) (Other :type Actor%20Object%20Reference) (OtherComp :type Primitive%20Component%20Object%20Reference) (bSelfMoved :type Boolean) (HitLocation :type Vector :default "0, 0, 0") (HitNormal :type Vector :default "0, 0, 0") (NormalImpulse :type Vector :default "0, 0, 0") (Hit :type Hit%20Result%20Structure%20%28by%20ref%29))
  ;[0.15 0.04642 0.0653 0.5] Trigger and Collision
)

(fn ConstructionScript)