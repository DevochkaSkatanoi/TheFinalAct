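; BP_Gravestone is a gravestone prop that randomizes its own appearance when play begins.
; BeginPlay applies a random height offset bounded above by MaxHight, a random tilt and yaw, and non-uniform scene scale.
; A random integer switch then sets the mesh to a cylinder, cone or cube.
; Construction script, overlap and tick do nothing, and an alternative random-mesh node is left unconnected.
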(event EventBeginPlay
  (bind _returnvalue (Math|Random|RandomFloatinRange -2e+01 2e+01))
  (bind _returnvalue_2 (Math|Random|RandomFloatinRange 0.8 1.2))
  (bind _gravestone_1 (Variables|Default|GetGravestone_1))
  ;[0.15 0.15 0.15 0.5] z-location
  (Transformation|AddWorldOffset (Variables|Default|GetGravestone_1) (Math|Vector|MakeVector 0.0 0.0 (Math|Random|RandomFloatinRange (stale _result) (Variables|Default|GetMax_Hight))) false false)
  (Transformation|AddWorldRotation (Variables|Default|GetGravestone_1) (Math|Rotator|MakeRotator _returnvalue _returnvalue (Math|Random|RandomFloatinRange 2e+01 1.6e+02)) false false)
  (Transformation|SetWorldScale3D (Variables|Default|GetScene) (Math|Vector|MakeVector _returnvalue_2 _returnvalue_2 _returnvalue_2))
  (switch int (Math|Random|RandomIntegerinRange 0 2)
    (:0
      (Components|StaticMesh|SetStaticMesh _gravestone_1 "/Engine/BasicShapes/Cylinder.Cylinder"))
    (:1
      (Components|StaticMesh|SetStaticMesh _gravestone_1 "/Engine/BasicShapes/Cone.Cone"))
    (:2
      (Components|StaticMesh|SetStaticMesh _gravestone_1 "/Engine/BasicShapes/Cube.Cube"))))

(event Collision|EventActorBeginOverlap
  (params (OtherActor :type Actor%20Object%20Reference)))

(event EventTick
  (params (DeltaSeconds :type Float%20%28single-precision%29)))

(fn ConstructionScript)