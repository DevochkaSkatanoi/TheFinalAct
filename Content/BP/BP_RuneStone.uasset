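; BP_RuneStone is a rune stone that lights up when BP_Samael overlaps its sphere.
; The overlap plays a timeline whose emission curve, scaled by a maximum strength, drives the Emissive parameter on the mesh materials.
; When the timeline finishes, the stone flags itself as on and calls its TurnedOn event dispatcher.
; BeginPlay stores a dynamic material instance, but the glow is set through the mesh component directly.
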(event OnComponentBeginOverlap(Sphere)
  (params (OverlappedComponent :type Primitive%20Component%20Object%20Reference) (OtherActor :type Actor%20Object%20Reference) (OtherComp :type Primitive%20Component%20Object%20Reference) (OtherBodyIndex :type Integer) (bFromSweep :type Boolean) (SweepResult :type Hit%20Result%20Structure%20%28by%20ref%29))
  (Utilities|Casting|CastToBP_Samael OtherActor)
  (bind _emission (Timeline|Timeline Play)
    (:Update
      (Rendering|Material|SetScalarParameterValueonMaterials (Variables|Default|GetMesh) "Emissive" (* _emission (Variables|Default|GetMaxEmissiveStrengh))))
    (:Finished
      (Variables|Default|SetisOn true)
      (Default|CallOnTurnedon))))

(event EventBeginPlay
  (bind _returnvalue (Rendering|Material|CreateDynamicMaterialInstance (Variables|Default|GetMesh) 0 0 "None" :!class /Script/Engine.PrimitiveComponent))
  (Variables|Default|SetMID _returnvalue))

(fn ConstructionScript)