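; BP_MovingTrap is a moving trap that knocks the BP_Samael character away on contact.
; A timeline, rate-scaled by MovingSpeed and played from Tick, drives the pitch rotation of the Piviot component.
; When Cylinder1 hits BP_Samael, it launches the character horizontally away from the cylinder with a negative Z component, overriding existing velocity, and prints a debug message.
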(event OnComponentHit(Cylinder1)
  (params (HitComponent :type Primitive%20Component%20Object%20Reference) (OtherActor :type Actor%20Object%20Reference) (OtherComp :type Primitive%20Component%20Object%20Reference) (NormalImpulse :type Vector :default "0, 0, 0") (Hit :type Hit%20Result%20Structure%20%28by%20ref%29))
  (bind _asbp_samael (Utilities|Casting|CastToBP_Samael OtherActor))
  (Character|LaunchCharacter _asbp_samael (* (+ (Math|Vector|Normalize (Math|Vector|MakeVector (.x (- (Transformation|GetActorLocation _asbp_samael) (Transformation|GetWorldLocation (Variables|Default|GetCylinder1)))) (.y (- (Transformation|GetActorLocation _asbp_samael) (Transformation|GetWorldLocation (Variables|Default|GetCylinder1)))) 0.0)) "0.000000,0.000000,0.800000") "1000.000000,1000.000000,-1000.000000") true true)
  (Development|PrintString "Launch" true true "(R=1.000000,G=0.050363,B=0.000000,A=1.000000)"))

(event EventBeginPlay
  (Components|Timeline|SetPlayRate (Variables|Default|GetTimeline) (Variables|Default|GetMoving%20Speed)))

(event EventTick
  (params (DeltaSeconds :type Float%20%28single-precision%29))
  (bind _rotation (Timeline|Timeline Play)
    (:Update
      (Transformation|SetRelativeRotation (Variables|Default|GetPiviot) (Math|Rotator|MakeRotator 0.0 (* _rotation 1e+01) 0.0) false false))))

(fn ConstructionScript)