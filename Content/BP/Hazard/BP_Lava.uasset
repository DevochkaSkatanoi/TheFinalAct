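; BP_Lava is a rising lava hazard that respawns BP_Samael when the player character touches its Cube.
; LavaBeginnRise starts the LavaRise timeline after a delay, nudging the Cube upward by a scaled curve value each update.
; Contact stops the timeline, returns the Cube to StartPos with a debug print, then resumes rising after short delays.
; StartPos is captured at construction, and SetNewStartPose replaces it with a hard-coded height.
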(event OnComponentBeginOverlap(Cube)
  (params (OverlappedComponent :type Primitive%20Component%20Object%20Reference) (OtherActor :type Actor%20Object%20Reference) (OtherComp :type Primitive%20Component%20Object%20Reference) (OtherBodyIndex :type Integer) (bFromSweep :type Boolean) (SweepResult :type Hit%20Result%20Structure%20%28by%20ref%29))
  (bind _startpos (Variables|Default|GetStartPos))
  (bind _asbp_samael (Utilities|Casting|CastToBP_Samael OtherActor))
  (Default|Respawn _asbp_samael)
  (Audio|Components|Audio|Stop (Variables|Default|GetLavaRise))
  (Utilities|FlowControl|Delay 1.0)
  (Transformation|SetRelativeLocation (Variables|Default|GetCube) _startpos false false)
  (Development|PrintString (Utilities|String|ToString(Vector) _startpos) true true "(R=1.000000,G=0.007671,B=0.375063,A=1.000000)" 5.0)
  (Utilities|FlowControl|Delay 1.0)
  (Audio|Components|Audio|Play (Variables|Default|GetLavaRise)))

(event Custom|SetNewStartPose
  (Variables|Default|SetStartPos "0.000000,0.000000,770.511105"))

(event Custom|LavaBeginnRise
  (Utilities|FlowControl|Delay 2.0)
  (bind _lava_z (Timeline|LavaRise Play)
    (:Update
      (Transformation|AddRelativeLocation (Variables|Default|GetCube) (Math|Vector|MakeVector 0.0 0.0 (* _lava_z 0.2)) false false))))

(event Collision|EventActorBeginOverlap
  (params (OtherActor :type Actor%20Object%20Reference)))

(fn ConstructionScript
  (Variables|Default|SetStartPos (Variables|/Script/Engine.SceneComponent|GetRelativeLocation (Variables|Default|GetCube))))