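; Timed spike hazard that extends and retracts on a continuous cycle starting at BeginPlay.
; A FlipFlop alternates a timeline between playing forward and reversing, scaling its curve by MaxExtendDistance to set the pivot's relative Z.
; TriggerSpikeChange waits Unten before each move, and the timeline's Finished output waits Oben before calling it again, so both delays separate successive moves.
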(event Custom|TriggerSpikeChange
  (Utilities|FlowControl|Delay (Variables|Default|GetUnten))
  (Utilities|FlowControl|FlipFlop
    (:A
      (bind _extendp (Timeline|Timeline PlayFromStart)
        (:Update
          (Transformation|SetRelativeLocation (Variables|Default|GetPiviot) (Math|Vector|MakeVector 0.0 0.0 (* _extendp (Variables|Default|GetMaxExtendDistance))) false false))
        (:Finished
          (Utilities|FlowControl|Delay (Variables|Default|GetOben))
          (CallFunction|TriggerSpikeChange))))
    (:B
      (Timeline|Timeline ReverseFromEnd))))

(event EventBeginPlay
  (CallFunction|TriggerSpikeChange))

(fn ConstructionScript)