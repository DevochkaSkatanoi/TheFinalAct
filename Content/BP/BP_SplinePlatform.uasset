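; Moving platform actor that travels in a continuous loop along the spline of a referenced spline actor.
; Tick places it at the current distance, optionally matching spline rotation, then advances by Speed times delta time, wrapping past the end.
; The construction script also updates the transform, then sets the start distance from a fraction of spline length.
; A missing spline reference triggers a one-time on-screen warning in the transform update.
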(event Custom|Updatetransform
  ;[0.04098 0.04631 0.15 0.5] Update Transform
  (Utilities|IsValid (Variables|Default|GetSpline)
    (:Is%20Valid
      (CallFunction|TransformPos))
    (:Is%20Not%20Valid
      (Utilities|FlowControl|DoOnce false
        (:Completed
          (Development|PrintString "No spline assined" true true "(R=1.000000,G=0.011157,B=0.000000,A=1.000000)" 5.0))))))

(event EventBeginPlay)

(event Collision|EventActorBeginOverlap
  (params (OtherActor :type Actor%20Object%20Reference)))

(event EventTick
  (params (DeltaSeconds :type Float%20%28single-precision%29))
  (bind _spline (Variables|Default|GetSpline))
  (bind _spline_2 (Variables|/Game/BP/BP_Spline.BP_Spline_C|GetSpline _spline))
  (bind _returnvalue (Spline|GetSplineLength _spline_2))
  (CallFunction|Updatetransform)
  (Variables|Default|SetDistanceAlongSpline (+ (Variables|Default|GetDistanceAlongSpline) (* (Variables|Default|GetSpeed) (Utilities|Time|GetWorldDeltaSeconds))))
  (if (> (Variables|Default|GetDistanceAlongSpline) _returnvalue)
    (Variables|Default|SetDistanceAlongSpline (- (Variables|Default|GetDistanceAlongSpline) _returnvalue))))

(fn ConstructionScript
  (CallFunction|Updatetransform)
  (CallFunction|SetStartDistance))

(fn TransformPos
  (bind _spline (Variables|Default|GetSpline))
  (bind _distancealongspline (Variables|Default|GetDistanceAlongSpline))
  (bind _spline_2 (Variables|/Game/BP/BP_Spline.BP_Spline_C|GetSpline _spline))
  (bind _returnvalue (Spline|GetTransformatDistanceAlongSpline _spline_2 _distancealongspline "World" false))
  (Transformation|SetActorLocation (.location _returnvalue) false false)
  (if (Variables|Default|GetbRotateWith)
    (Transformation|SetActorRotation (.rotation _returnvalue))))

(fn SetStartDistance
  (bind _spline (Variables|Default|GetSpline))
  (Utilities|IsValid _spline
    (:Is%20Valid
      (Variables|Default|SetDistanceAlongSpline (* (Spline|GetSplineLength (Variables|/Game/BP/BP_Spline.BP_Spline_C|GetSpline _spline)) (Variables|Default|GetDistancePercentOnStart))))))