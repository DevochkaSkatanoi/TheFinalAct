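; BP_RuneGate is a gate that opens by moving a scene component vertically.
; Its Open event fires once, playing the OpenGate timeline whose track, scaled by a GateLocation variable, sets the component's relative Z.
; A check that all three rune stones are on before calling Open exists but is disconnected, and Tick is empty, so the gate relies on an outside call to Open.
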(event Custom|Open
  (Utilities|FlowControl|DoOnce false
    (:Completed
      (bind _gatelocation (Timeline|OpenGate Play)
        (:Update
          (Transformation|SetRelativeLocation (Variables|Default|GetScene1) (Math|Vector|MakeVector 0.0 0.0 (* _gatelocation (Variables|Default|GetGateLocation))) false false))))))

(event EventTick
  (params (DeltaSeconds :type Float%20%28single-precision%29)))

(fn ConstructionScript)