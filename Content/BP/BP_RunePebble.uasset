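; BP_RunePebble is a rune pebble mesh whose glow strengthens as the player character approaches.
; Every tick it maps the player-to-mesh distance to a clamped Emissive scalar parameter on the mesh materials, brightest up close.
; BeginPlay creates and stores a dynamic material instance, though Tick sets the parameter through the mesh component.
; A separate custom event, not called within this graph, gives the mesh a random world rotation.
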(event Custom|RandomRotatiom
  ;[0.15 0.03383 0.05567 0.5] Random Rotation
  (Transformation|SetWorldRotation (Variables|Default|GetMesh) (Math|Rotator|MakeRotator (Math|Random|RandomFloatinRange 0.0 3.6e+02) (Math|Random|RandomFloatinRange 0.0 3.6e+02) (Math|Random|RandomFloatinRange 0.0 3.6e+02)) false false))

(event EventBeginPlay
  (bind _returnvalue (Rendering|Material|CreateDynamicMaterialInstance (Variables|Default|GetMesh) 0 0 "None" :!class /Script/Engine.PrimitiveComponent))
  (Variables|Default|SetMID _returnvalue))

(event EventTick
  (params (DeltaSeconds :type Float%20%28single-precision%29))
  (Rendering|Material|SetScalarParameterValueonMaterials (Variables|Default|GetMesh) "Emissive" (Math|Float|MapRangeClamped (Math|Vector|VectorLength (- (Transformation|GetWorldLocation (Variables|Default|GetMesh)) (Transformation|GetActorLocation (Game|GetPlayerCharacter 0)))) 2e+03 2e+02 0.0 1e+02)))

(fn ConstructionScript)